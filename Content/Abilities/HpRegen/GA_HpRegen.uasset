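; GA_HpRegen is a gameplay ability that toggles HP regen Allowed/DisAllowed tags and handles the owner's death.
; An upper-threshold watcher feeds paired gates that switch tags once per crossing, applying GE_HpMax on reaching it.
; A lower-threshold watcher calls Die on ThirdPersonCharacterSimple and ends all watchers.
; An attribute-change watcher rescales the actor by square root and restarts the upper watcher with a fresh threshold.
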(event `self.K2_ActivateAbility`
  (bind _returnvalue (`BlueprintGameplayTagLibrary.MakeLiteralGameplayTagContainer` (struct :`GameplayTags` (struct :`(TagName` "GA.HpRegen.DisAllowed")))))
  (bind _returnvalue_2 (`BlueprintGameplayTagLibrary.MakeLiteralGameplayTagContainer` (struct :`GameplayTags` (struct :`(TagName` "GA.HpRegen.Allowed")))))
  (bind _returnvalue_3 (`self.GetOwningActorFromActorInfo`))
  (bind _returnvalue_4 (`self.GetOwningActorFromActorInfo`))
  (bind _returnvalue_5 (`self.GetOwningActorFromActorInfo`))
  (bind _async_task_0 (`self.Async Task_0`))
  (bind _async_task (`self.Async Task`))
  (bind _async_task_1 (`self.Async Task_1`))
  (`|ExecutionSequence`
    (:`then_0`
      (bind (_asynctaskproxy _bmatchescomparison) (`AbilityTask_WaitAttributeChangeThreshold.WaitForAttributeChangeThreshold` (struct :`AttributeName` "Health" :`Attribute` "/Script/GAS.GASAttributeSet:Health" :`AttributeOwner` "/Script/CoreUObject.Class'\"/Script/GAS.GASAttributeSet\"'") "GreaterThanOrEqualTo" (`.ReturnValue` (`AbilitySystemBlueprintLibrary.GetFloatAttribute` _returnvalue_4 (struct :`AttributeName` "HealthMax" :`Attribute` "/Script/GAS.GASAttributeSet:HealthMax" :`AttributeOwner` "/Script/CoreUObject.Class'\"/Script/GAS.GASAttributeSet\"'"))) false _returnvalue_4 :!label _label)
        (:`then`
          (set `self.Async Task` _asynctaskproxy))
        (:`OnChange`
          (if _bmatchescomparison
            (`|ExecutionSequence`
              (:`then_0`
                (`/Engine/EditorBlueprintResources/StandardMacros.Gate` true :!label _label_2
                  (:`Exit`
                    (`AbilitySystemBlueprintLibrary.RemoveLooseGameplayTags` _returnvalue_5 _returnvalue_2)
                    (`AbilitySystemBlueprintLibrary.AddLooseGameplayTags` _returnvalue_5 _returnvalue)
                    (`self.BP_ApplyGameplayEffectToOwner` "/Game/Abilities/HpRegen/GE_HpMax.GE_HpMax_C"))))
              (:`then_1`
                (goto _label_2 :!via `Close`))
              (:`then_2`
                (goto _label_3 :!via `Open`)))
            (else
              (`|ExecutionSequence`
                (:`then_0`
                  (`/Engine/EditorBlueprintResources/StandardMacros.Gate` true :!label _label_3
                    (:`Exit`
                      (`AbilitySystemBlueprintLibrary.AddLooseGameplayTags` _returnvalue_5 _returnvalue_2)
                      (`AbilitySystemBlueprintLibrary.RemoveLooseGameplayTags` _returnvalue_5 _returnvalue))))
                (:`then_1`
                  (goto _label_3 :!via `Close`))
                (:`then_2`
                  (goto _label_2 :!via `Open`))))))))
    (:`then_1`
      (bind (_asynctaskproxy_2 _bmatchescomparison_2) (`AbilityTask_WaitAttributeChangeThreshold.WaitForAttributeChangeThreshold` (struct :`AttributeName` "Health" :`Attribute` "/Script/GAS.GASAttributeSet:Health" :`AttributeOwner` "/Script/CoreUObject.Class'\"/Script/GAS.GASAttributeSet\"'") "LessThanOrEqualTo" 0.0 false _returnvalue_4)
        (:`then`
          (set `self.Async Task_0` _asynctaskproxy_2))
        (:`OnChange`
          (if _bmatchescomparison_2
            (`|ExecutionSequence`
              (:`then_0`
                (goto _label_2 :!via `Close`))
              (:`then_1`
                (goto _label_3 :!via `Close`))
              (:`then_2`
                (`AbilitySystemBlueprintLibrary.RemoveLooseGameplayTags` _returnvalue_5 _returnvalue_2)
                (`AbilitySystemBlueprintLibrary.AddLooseGameplayTags` _returnvalue_5 _returnvalue)
                (bind _asthird_person_character (cast `/Game/ThirdPersonCPP/Blueprints/ThirdPersonCharacterSimple` _returnvalue_5))
                (`/Game/ThirdPersonCPP/Blueprints/ThirdPersonCharacterSimple.Die` _asthird_person_character))
              (:`then_3`
                (`/Engine/EditorBlueprintResources/StandardMacros.IsValid` _async_task :!label _label_4
                  (:`Is Valid`
                    (`GameplayTask.EndTask` _async_task))))
              (:`then_4`
                (`/Engine/EditorBlueprintResources/StandardMacros.IsValid` _async_task_0
                  (:`Is Valid`
                    (`GameplayTask.EndTask` _async_task_0))))
              (:`then_5`
                (`/Engine/EditorBlueprintResources/StandardMacros.IsValid` _async_task_1
                  (:`Is Valid`
                    (`GameplayTask.EndTask` _async_task_1)))))))))
    (:`then_2`
      (bind _asynctaskproxy_3 (`AbilityTask_WaitAttributeChange.WaitForAttributeChange` (struct :`AttributeName` "HealthMax" :`Attribute` "/Script/GAS.GASAttributeSet:HealthMax" :`AttributeOwner` "/Script/CoreUObject.Class'\"/Script/GAS.GASAttributeSet\"'") (struct) (struct) false null)
        (:`then`
          (set `self.Async Task_1` _asynctaskproxy_3))
        (:`OnChange`
          (`Actor.SetActorScale3D` _returnvalue_3 (`KismetMathLibrary.Conv_DoubleToVector` (`KismetMathLibrary.MultiplyMultiply_FloatFloat` (/ (`.ReturnValue` (`AbilitySystemBlueprintLibrary.GetFloatAttribute` _returnvalue_3 (struct :`AttributeName` "HealthMax" :`Attribute` "/Script/GAS.GASAttributeSet:HealthMax" :`AttributeOwner` "/Script/CoreUObject.Class'\"/Script/GAS.GASAttributeSet\"'"))) 100.0) 0.5)))
          (`|ExecutionSequence`
            (:`then_0`
              (goto _label_4))
            (:`then_1`
              (goto _label))))))))