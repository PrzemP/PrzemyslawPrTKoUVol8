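; BP_GeneralProjectile is a homing ability projectile that delivers a gameplay effect to a specific target.
; On BeginPlay it homes on the target's capsule, then opens a gate after a short delay.
; Actor or Sphere1 overlap with the target applies GEForTarget through the target's Ability System Component and destroys the projectile.
; Other overlaps destroy it only once the gate is open, so early contacts are ignored.
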(event `self.ReceiveBeginPlay`
  (set `ProjectileMovementComponent.HomingTargetComponent` (`Character.CapsuleComponent` (`self.Target`)) (`self.ProjectileMovement`))
  (`KismetSystemLibrary.Delay` 0.1)
  (goto _label_2 :!via `Open`))

(event `self.ReceiveActorBeginOverlap`
  (params (OtherActor :type "Actor Object Reference"))
  (bind _target (`self.Target`))
  (if (== _target OtherActor)
    (`AbilitySystemComponent.BP_ApplyGameplayEffectSpecToSelf` (`AbilitySystemBlueprintLibrary.GetAbilitySystemComponent` _target) (`self.GE for target`) :!label _label)
    (else
      (`/Engine/EditorBlueprintResources/StandardMacros.Gate` true :!label _label_2
        (:`Exit`
          _))))
  (`self.K2_DestroyActor` self))

(event `self.Sphere1.OnComponentBeginOverlap`
  (params (OverlappedComponent :type "PrimitiveComponent Object Reference") (OtherActor :type "Actor Object Reference") (OtherComp :type "PrimitiveComponent Object Reference") (OtherBodyIndex :type Integer) (bFromSweep :type Boolean) (SweepResult :type "HitResult Structure (by ref)"))
  (if (== (`self.Target`) OtherActor)
    (goto _label)
    (else
      (goto _label_2))))

(fn `UserConstructionScript`)