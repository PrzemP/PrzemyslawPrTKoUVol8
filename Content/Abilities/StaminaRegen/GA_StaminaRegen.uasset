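; Gameplay ability that switches stamina regeneration on and off with loose GA.StaminaRegen tags on the owner.
; An attribute threshold task at 100 drives two alternating gates, so each crossing fires once: reaching it blocks regen and applies GE_StaminaMax, dropping below allows regen.
; A second, lower-bound threshold task closes both gates, blocks regen, calls Die on the ThirdPersonCharacterSimple owner and ends both tasks.
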(event `self.K2_ActivateAbility`
  (bind _returnvalue (`BlueprintGameplayTagLibrary.MakeLiteralGameplayTagContainer` (struct :`GameplayTags` (struct :`(TagName` "GA.StaminaRegen.DIsAllowed")))))
  (bind _returnvalue_2 (`BlueprintGameplayTagLibrary.MakeLiteralGameplayTagContainer` (struct :`GameplayTags` (struct :`(TagName` "GA.StaminaRegen.Allowed")))))
  (bind _returnvalue_3 (`self.GetOwningActorFromActorInfo`))
  (bind _async_task (`self.Async Task`))
  (bind _async_task_0 (`self.Async Task_0`))
  (bind (_asynctaskproxy _bmatchescomparison) (`AbilityTask_WaitAttributeChangeThreshold.WaitForAttributeChangeThreshold` (struct :`AttributeName` "Stamina" :`Attribute` "/Script/GAS.GASAttributeSet:Stamina" :`AttributeOwner` "/Script/CoreUObject.Class'\"/Script/GAS.GASAttributeSet\"'") "GreaterThanOrEqualTo" 100.0 false null)
    (:`then`
      (set `self.Async Task` _asynctaskproxy)
      (bind (_asynctaskproxy_2 _bmatchescomparison_2) (`AbilityTask_WaitAttributeChangeThreshold.WaitForAttributeChangeThreshold` (struct :`AttributeName` "Health" :`Attribute` "/Script/GAS.GASAttributeSet:Health" :`AttributeOwner` "/Script/CoreUObject.Class'\"/Script/GAS.GASAttributeSet\"'") "LessThanOrEqualTo" 0.0 false null)
        (:`then`
          (set `self.Async Task_0` _asynctaskproxy_2))
        (:`OnChange`
          (if _bmatchescomparison_2
            (`|ExecutionSequence`
              (:`then_0`
                (goto _label :!via `Close`))
              (:`then_1`
                (goto _label_2 :!via `Close`))
              (:`then_2`
                (`AbilitySystemBlueprintLibrary.RemoveLooseGameplayTags` _returnvalue_3 _returnvalue_2)
                (`AbilitySystemBlueprintLibrary.AddLooseGameplayTags` _returnvalue_3 _returnvalue)
                (bind _asthird_person_character (cast `/Game/ThirdPersonCPP/Blueprints/ThirdPersonCharacterSimple` _returnvalue_3))
                (`/Game/ThirdPersonCPP/Blueprints/ThirdPersonCharacterSimple.Die` _asthird_person_character))
              (:`then_3`
                (`/Engine/EditorBlueprintResources/StandardMacros.IsValid` _async_task
                  (:`Is Valid`
                    (`GameplayTask.EndTask` _async_task))))
              (:`then_4`
                (`/Engine/EditorBlueprintResources/StandardMacros.IsValid` _async_task_0
                  (:`Is Valid`
                    (`GameplayTask.EndTask` _async_task_0)))))))))
    (:`OnChange`
      (if _bmatchescomparison
        (`|ExecutionSequence`
          (:`then_0`
            (`/Engine/EditorBlueprintResources/StandardMacros.Gate` true :!label _label
              (:`Exit`
                (`AbilitySystemBlueprintLibrary.RemoveLooseGameplayTags` _returnvalue_3 _returnvalue_2)
                (`AbilitySystemBlueprintLibrary.AddLooseGameplayTags` _returnvalue_3 _returnvalue)
                (`self.BP_ApplyGameplayEffectToOwner` "/Game/Abilities/StaminaRegen/GE_StaminaMax.GE_StaminaMax_C"))))
          (:`then_1`
            (goto _label :!via `Close`))
          (:`then_2`
            (goto _label_2 :!via `Open`)))
        (else
          (`|ExecutionSequence`
            (:`then_0`
              (`/Engine/EditorBlueprintResources/StandardMacros.Gate` true :!label _label_2
                (:`Exit`
                  (`AbilitySystemBlueprintLibrary.AddLooseGameplayTags` _returnvalue_3 _returnvalue_2)
                  (`AbilitySystemBlueprintLibrary.RemoveLooseGameplayTags` _returnvalue_3 _returnvalue))))
            (:`then_1`
              (goto _label_2 :!via `Close`))
            (:`then_2`
              (goto _label :!via `Open`))))))))