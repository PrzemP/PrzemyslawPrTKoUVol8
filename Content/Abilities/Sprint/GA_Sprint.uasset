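; GA_Sprint is a Gameplay Ability that makes the owning character sprint while the input is held.
; On activation it adds a replicated GA.Sprint.Allowed tag and multiplies MaxWalkSpeed by RunningSpeedMult, guarded by a DoOnce.
; Async tasks end the ability on input release or when a watched attribute stops exceeding its threshold.
; Ending resets the guard, stops both tasks, removes the tag and divides the speed back down.
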(event `self.K2_ActivateAbility`
  (bind _returnvalue (`Actor.GetComponentByClass` (`self.GetOwningActorFromActorInfo`) "/Script/Engine.CharacterMovementComponent"))
  (bind (_asynctaskproxy _bmatchescomparison) (`AbilityTask_WaitAttributeChangeThreshold.WaitForAttributeChangeThreshold` (struct :`AttributeName` "Stamina" :`Attribute` "/Script/GAS.GASAttributeSet:Stamina" :`AttributeOwner` "Class'\"/Script/GAS.GASAttributeSet\"'") "GreaterThan" 1.0 false null)
    (:`then`
      (set `self.Async Task` _asynctaskproxy)
      (bind _asynctaskproxy_2 (`AbilityTask_WaitInputRelease.WaitInputRelease` false)
        (:`then`
          (set `self.Async Task_0` _asynctaskproxy_2)
          (`/Engine/EditorBlueprintResources/StandardMacros.DoOnce` false :!label _label
            (:`Completed`
              (`AbilitySystemBlueprintLibrary.AddLooseGameplayTags` (`self.GetOwningActorFromActorInfo`) (`BlueprintGameplayTagLibrary.MakeLiteralGameplayTagContainer` (struct :`GameplayTags` (struct :`(TagName` "GA.Sprint.Allowed")))) true)
              (set `CharacterMovementComponent.MaxWalkSpeed` (* (`CharacterMovementComponent.MaxWalkSpeed` _returnvalue) (`self.RunningSpeedMult`)) _returnvalue))))
        (:`OnRelease`
          (`self.K2_EndAbility` :!label _label_2))))
    (:`OnChange`
      (if (not _bmatchescomparison)
        (goto _label_2)))))

(event `self.K2_OnEndAbility`
  (params (bWasCancelled :type Boolean))
  (bind _async_task (`self.Async Task`))
  (bind _async_task_0 (`self.Async Task_0`))
  (bind _returnvalue (`Actor.GetComponentByClass` (`self.GetOwningActorFromActorInfo`) "/Script/Engine.CharacterMovementComponent"))
  (`|ExecutionSequence`
    (:`then_0`
      (goto _label :!via `Reset`))
    (:`then_1`
      (`/Engine/EditorBlueprintResources/StandardMacros.IsValid` _async_task
        (:`Is Valid`
          (`GameplayTask.EndTask` _async_task))))
    (:`then_2`
      (`/Engine/EditorBlueprintResources/StandardMacros.IsValid` _async_task_0
        (:`Is Valid`
          (`GameplayTask.EndTask` _async_task_0))))
    (:`then_3`
      (`AbilitySystemBlueprintLibrary.RemoveLooseGameplayTags` (`self.GetOwningActorFromActorInfo`) (`BlueprintGameplayTagLibrary.MakeLiteralGameplayTagContainer` (struct :`GameplayTags` (struct :`(TagName` "GA.Sprint.Allowed")))) true)
      (set `CharacterMovementComponent.MaxWalkSpeed` (/ (`CharacterMovementComponent.MaxWalkSpeed` _returnvalue) (`self.RunningSpeedMult`)) _returnvalue))))