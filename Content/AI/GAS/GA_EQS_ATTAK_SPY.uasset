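; Gameplay Ability for an AI spy's close-range attack on other bots.
; A sphere overlap just in front of the owner picks a random BP_BotV2, records the attacker as DamagedBy in the victim's blackboard, applies SetByCaller damage and reports a damage event.
; Whether or not it hits, the owner then gets a short cooldown effect with dynamically granted tags and the ability ends immediately.
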(event `self.K2_ActivateAbility`
  (bind _returnvalue (`self.GetOwningActorFromActorInfo`))
  (bind _returnvalue_2 (`self.GetOwningActorFromActorInfo`))
  (`|ExecutionSequence`
    (:`then_0`
      (bind (_outactors _returnvalue_3) (`KismetSystemLibrary.SphereOverlapActors` (+ (`Actor.K2_GetActorLocation` _returnvalue) (* (`Actor.GetActorForwardVector` _returnvalue) 50.0)) 100.0 (`|MakeArray` "ObjectTypeQuery3" :!type "EObjectTypeQuery Enum") "/Game/AI/BP_BotV2.BP_BotV2_C" (`|MakeArray` _returnvalue)))
      (if _returnvalue_3
        (bind _output_get (set `self.Target` (`KismetArrayLibrary.Array_Random` _outactors)))
        (`BlackboardComponent.SetValueAsObject` (`AIBlueprintHelperLibrary.GetBlackboard` (`AIBlueprintHelperLibrary.GetAIController` (`self.Target`))) "DamagedBy" (`self.GetOwningActorFromActorInfo`))
        (bind _returnvalue_4 (`AbilitySystemBlueprintLibrary.GetAbilitySystemComponent` _output_get))
        ;[1 1 1] Bug fix spy kill with one hit
        (bind _returnvalue_5 (`AbilitySystemBlueprintLibrary.AssignTagSetByCallerMagnitude` (`AbilitySystemComponent.MakeOutgoingSpec` :`self` _returnvalue_4 :`GameplayEffectClass` "/Game/AI/GAS/GE_EQS_Deal_Damage.GE_EQS_Deal_Damage_C" :`Level` 1.0) (struct :`TagName` "EQS.DATA.P1") -100.0))
        (`AbilitySystemComponent.BP_ApplyGameplayEffectSpecToSelf` _returnvalue_4 _returnvalue_5)
        (`AISense_Damage.ReportDamageEvent` (`self.Target`) _returnvalue_2 10.0 (`Actor.K2_GetActorLocation` _returnvalue_2))))
    (:`then_1`
      (bind _returnvalue_6 (`AbilitySystemBlueprintLibrary.SetDuration` (`AbilitySystemComponent.MakeOutgoingSpec` :`self` (`AbilitySystemBlueprintLibrary.GetAbilitySystemComponent` (`self.GetOwningActorFromActorInfo`)) :`GameplayEffectClass` "/Game/AI/GAS/GE_EQS_COOLDOWN.GE_EQS_COOLDOWN_C" :`Level` 1.0) 1.0))
      (bind _returnvalue_7 (`AbilitySystemBlueprintLibrary.AddGrantedTags` _returnvalue_6 (`self.New Gameplay Tags`)))
      (`AbilitySystemComponent.BP_ApplyGameplayEffectSpecToSelf` (`AbilitySystemBlueprintLibrary.GetAbilitySystemComponent` (`self.GetOwningActorFromActorInfo`)) _returnvalue_7))
    (:`then_2`
      (`self.K2_EndAbility`))))