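; Gameplay ability that fires a sniper shot from an AI pawn at its blackboard ActorTarget.
; It spawns a BP_BotBullet just ahead of the pawn, rotated toward the target, passing owner data and a projectile type chosen from the blackboard's SelectedAmmoName.
; It then applies GE_EQS_COOLDOWN to itself with a runtime-set duration and granted tags, and ends immediately.
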(event `self.K2_ActivateAbility`
  (bind _returnvalue (`self.GetOwningActorFromActorInfo`))
  (bind _returnvalue_location (`KismetMathLibrary.BreakTransform` (`Actor.GetTransform` _returnvalue)))
  (bind _returnvalue_2 (`AIBlueprintHelperLibrary.GetBlackboard` _returnvalue))
  (bind _returnvalue_3 (`BlackboardComponent.GetValueAsName` _returnvalue_2 "SelectedAmmoName"))
  (bind _returnvalue_4 (+ (`Actor.GetActorForwardVector` _returnvalue) _returnvalue_location))
  (`|ExecutionSequence`
    (:`then_0`
      (bind _asactor (cast `Actor` (`BlackboardComponent.GetValueAsObject` _returnvalue_2 "ActorTarget")))
      (bind _aspawn (cast `Pawn` (`self.GetOwningActorFromActorInfo`)))
      (bind _returnvalue_location_2 (`KismetMathLibrary.BreakTransform` (`Actor.GetTransform` _asactor)))
      (`|SpawnActorFromClass` "/Game/AI/BP_BotBullet.BP_BotBullet_C" (`KismetMathLibrary.MakeTransform` _returnvalue_4 (`KismetMathLibrary.FindLookAtRotation` _returnvalue_4 _returnvalue_location_2)) "Undefined" "OverrideRootScale" _aspawn (`AbilitySystemBlueprintLibrary.GetAbilitySystemComponent` _aspawn) 1000.0 null "NewEnumerator2" (select `bool` (== _returnvalue_3 "Slow") :`false` (select `bool` (== _returnvalue_3 "Fast") :`false` "NewEnumerator2" :`true` "NewEnumerator1" :!type "/Game/AI/E_SNIPER_AMMO Enum") :`true` "NewEnumerator0") 5000.0 _aspawn))
    (:`then_1`
      (bind _returnvalue_5 (`AbilitySystemBlueprintLibrary.SetDuration` (`AbilitySystemComponent.MakeOutgoingSpec` :`self` (`AbilitySystemBlueprintLibrary.GetAbilitySystemComponent` (`self.GetOwningActorFromActorInfo`)) :`GameplayEffectClass` "/Game/AI/GAS/GE_EQS_COOLDOWN.GE_EQS_COOLDOWN_C" :`Level` 1.0) 1.0))
      (bind _returnvalue_6 (`AbilitySystemBlueprintLibrary.AddGrantedTags` _returnvalue_5 (`self.New Gameplay Tags`)))
      (`AbilitySystemComponent.BP_ApplyGameplayEffectSpecToSelf` (`AbilitySystemBlueprintLibrary.GetAbilitySystemComponent` (`self.GetOwningActorFromActorInfo`)) _returnvalue_6))
    (:`then_2`
      (`self.K2_EndAbility`))))