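; Gameplay Ability for the AI pyro attack, firing a BP_BotBullet at the blackboard's ActorTarget.
; On activation it spawns the bullet just ahead of the owning pawn, rotated toward the target, passing owner, ability system and class.
; It then self-applies GE_EQS_COOLDOWN with a very short overridden duration and added granted tags, and ends immediately.
; A failed target or pawn cast skips only the shot.
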(event `self.K2_ActivateAbility`
  (bind _returnvalue (`self.GetOwningActorFromActorInfo`))
  (bind _returnvalue_location (`KismetMathLibrary.BreakTransform` (`Actor.GetTransform` _returnvalue)))
  (bind _returnvalue_2 (+ (`Actor.GetActorForwardVector` _returnvalue) _returnvalue_location))
  (`|ExecutionSequence`
    (:`then_0`
      (bind _asactor (cast `Actor` (`BlackboardComponent.GetValueAsObject` (`AIBlueprintHelperLibrary.GetBlackboard` _returnvalue) "ActorTarget")))
      (bind _aspawn (cast `Pawn` (`self.GetOwningActorFromActorInfo`)))
      (bind _returnvalue_location_2 (`KismetMathLibrary.BreakTransform` (`Actor.GetTransform` _asactor)))
      (`|SpawnActorFromClass` "/Game/AI/BP_BotBullet.BP_BotBullet_C" (`KismetMathLibrary.MakeTransform` _returnvalue_2 (`KismetMathLibrary.FindLookAtRotation` _returnvalue_2 _returnvalue_location_2)) "Undefined" "OverrideRootScale" _aspawn (`AbilitySystemBlueprintLibrary.GetAbilitySystemComponent` _aspawn) 1000.0 null "NewEnumerator1" "NewEnumerator0" _aspawn))
    (:`then_1`
      (bind _returnvalue_3 (`AbilitySystemBlueprintLibrary.SetDuration` (`AbilitySystemComponent.MakeOutgoingSpec` :`self` (`AbilitySystemBlueprintLibrary.GetAbilitySystemComponent` (`self.GetOwningActorFromActorInfo`)) :`GameplayEffectClass` "/Game/AI/GAS/GE_EQS_COOLDOWN.GE_EQS_COOLDOWN_C" :`Level` 1.0) 0.01))
      (bind _returnvalue_4 (`AbilitySystemBlueprintLibrary.AddGrantedTags` _returnvalue_3 (`self.New Gameplay Tags`)))
      (`AbilitySystemComponent.BP_ApplyGameplayEffectSpecToSelf` (`AbilitySystemBlueprintLibrary.GetAbilitySystemComponent` (`self.GetOwningActorFromActorInfo`)) _returnvalue_4))
    (:`then_2`
      (`self.K2_EndAbility`))))