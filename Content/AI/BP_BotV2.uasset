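; BP_BotV2 is a class-based AI bot character (Balance, Pyro, Sniper or Spy) built on the Gameplay Ability System.
; The construction script picks the AI controller from Class.
; BeginPlay applies EQS init, class-specific (none for Balance) and character default gameplay effects, and sets a team material for positive TeamIDs.
; An attribute watcher spawns a death mark and destroys the bot when the value reaches zero or below.
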(event `self.ReceiveBeginPlay`
  (`|ExecutionSequence`
    (:`then_0`
      (`AbilitySystemComponent.BP_ApplyGameplayEffectToSelf` :`self` (`self.AbilitySystemComponent`) :`GameplayEffectClass` "/Game/AI/GAS/GE_EQS_Init.GE_EQS_Init_C" :`Level` 1.0))
    (:`then_1`
      (switch `/Game/AI/E_BotClass` (`self.Class`)
        (:`NewEnumerator1`
          (`AbilitySystemComponent.BP_ApplyGameplayEffectToSelf` :`self` (`self.AbilitySystemComponent`) :`GameplayEffectClass` "/Game/AI/GAS/GE_EQS_CLASS_Pyro.GE_EQS_CLASS_Pyro_C" :`Level` 1.0))
        (:`NewEnumerator2`
          (`AbilitySystemComponent.BP_ApplyGameplayEffectToSelf` :`self` (`self.AbilitySystemComponent`) :`GameplayEffectClass` "/Game/AI/GAS/GE_EQS_CLASS_Sniper.GE_EQS_CLASS_Sniper_C" :`Level` 1.0))
        (:`NewEnumerator3`
          (`AbilitySystemComponent.BP_ApplyGameplayEffectToSelf` :`self` (`self.AbilitySystemComponent`) :`GameplayEffectClass` "/Game/AI/GAS/GE_EQS_CLASS_Spy.GE_EQS_CLASS_Spy_C" :`Level` 1.0))))
    (:`then_2`
      (`AbilitySystemComponent.BP_ApplyGameplayEffectToSelf` :`self` (`self.AbilitySystemComponent`) :`GameplayEffectClass` "/Game/Abilities/GE_CharacterDefaults.GE_CharacterDefaults_C" :`Level` 1.0)
      (bind (_asynctaskproxy _attribute _newvalue) (`AbilityAsync_WaitAttributeChanged.WaitForAttributeChanged` null (struct :`AttributeName` "Health" :`Attribute` "/Script/GAS.GASAttributeSet:Health" :`AttributeOwner` "/Script/CoreUObject.Class'\"/Script/GAS.GASAttributeSet\"'"))
        (:`Changed`
          (if (<= _newvalue 0.0)
            (`|SpawnActorFromClass` "/Game/AI/Props/BP_DeathMark.BP_DeathMark_C" (`self.GetTransform`) "Undefined" "MultiplyWithRoot" null null)
            (`self.K2_DestroyActor`)))))
    (:`then_3`
      (if (> (`self.TeamID`) 0)
        (`PrimitiveComponent.SetMaterial` (`self.Mesh`) 0 (`|GetArrayItem` (`self.Colors`) (`self.TeamID`)))))))

(fn `UserConstructionScript`
  (switch `/Game/AI/E_BotClass` (`self.Class`)
    (:`NewEnumerator0`
      (set `self.AIControllerClass` "/Game/AI/BOTS/BALANCE/AIC_Bot_BALANCE.AIC_Bot_BALANCE_C"))
    (:`NewEnumerator1`
      (set `self.AIControllerClass` "/Game/AI/BOTS/PYRO/AIC_Bot_PYRO.AIC_Bot_PYRO_C"))
    (:`NewEnumerator2`
      (set `self.AIControllerClass` "/Game/AI/BOTS/SNIPER/AIC_Bot_SNIPER.AIC_Bot_SNIPER_C"))
    (:`NewEnumerator3`
      (set `self.AIControllerClass` "/Game/AI/BOTS/SPY/AIC_Bot_SPY.AIC_Bot_SPY_C"))))